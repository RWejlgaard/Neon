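; Enemy AI pawn that chases the player, deals melee damage on a short cooldown and destroys itself when HP runs out.
; Until annoyed, it sweeps a line trace around itself, one degree per Tick.
; A trace hit on the player or any damage taken makes it annoyed, enabling pursuit and close-range attacks.
; Attack turns its spotlight red and calls SimpleMoveToActor; PawnSensing also triggers it, without setting Annoyed.
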(event OnSeePawn(PawnSensing)
  (params (Pawn :type Pawn%20Object%20Reference))
  (CallFunction|Attack))

(event EventTick
  (params (DeltaSeconds :type Float%20%28single-precision%29))
  (if (<= (Variables|Default|GetHP) 0)
    (CallFunction|Die)
    (elif (Variables|Default|Getannoyed)
      (if (< (Transformation|GetDistanceTo (Game|GetPlayerCharacter 0)) 1.2e+02)
        (if (not (Variables|Default|GetisHot))
          (Game|Damage|ApplyDamage (Game|Player|GetPlayerPawn 0) 5.0 0 self)
          (Variables|Default|SetisHot true)
          (Utilities|FlowControl|Delay 0.5)
          (Variables|Default|SetisHot false))
        (else
          (CallFunction|Attack)))
      (else
        (CallFunction|ScanTick)))))

(event Game|Damage|EventAnyDamage
  (params (Damage :type Float%20%28single-precision%29) (DamageType :type Damage%20Type%20Object%20Reference) (InstigatedBy :type Controller%20Object%20Reference) (DamageCauser :type Actor%20Object%20Reference))
  (CallFunction|GetAnnoyed)
  (if (<= (Variables|Default|GetHP) 0)
    (CallFunction|Die)
    (else
      (bind _output_get (Variables|Default|SetHP (- (Variables|Default|GetHP) (Math|Float|Floor Damage))))
      (Development|PrintString (Utilities|String|ToString(Integer) _output_get))
      (if (< _output_get 0)
        _))))

(event Collision|EventHit
  (params (MyComp :type Primitive%20Component%20Object%20Reference) (Other :type Actor%20Object%20Reference) (OtherComp :type Primitive%20Component%20Object%20Reference) (bSelfMoved :type Boolean) (HitLocation :type Vector :default "0, 0, 0") (HitNormal :type Vector :default "0, 0, 0") (NormalImpulse :type Vector :default "0, 0, 0") (Hit :type Hit%20Result%20Structure%20%28by%20ref%29)))

(fn ConstructionScript)

(fn Attack
  (Rendering|Components|Light|SetLightColor (Variables|Default|GetSpotLight) "(R=1.000000,G=0.000000,B=0.000000,A=1.000000)" true)
  (AI|Navigation|SimpleMovetoActor (Pawn|GetController) (Game|GetPlayerCharacter 0)))

(fn Die
  (Actor|DestroyActor))

(fn LookforPlayer
  (if (Variables|/Script/AIModule.PawnSensingComponent|GetbSeePawns (Variables|Default|GetPawnSensing))
    (CallFunction|Attack)))

(fn GetAnnoyed
  (Variables|Default|Setannoyed true))

(fn ScanTick
  (bind _capsulecomponent (Variables|Collision|GetCapsuleComponent))
  (bind _returnvalue (Transformation|GetWorldLocation _capsulecomponent))
  (bind _returnvalue_2 (Transformation|GetWorldRotation _capsulecomponent))
  (bind (_x _y _z) (Math|Vector|BreakVector _returnvalue))
  (bind (_roll _pitch) (Math|Rotator|BreakRotator _returnvalue_2))
  (bind _returnvalue_3 (Math|Vector|MakeVector _x _y _z))
  (bind _outhit (Collision|LineTraceByChannel _returnvalue_3 (+ (* (Math|Vector|GetForwardVector (Math|Rotator|MakeRotator _roll _pitch (Variables|Default|GetscanRotation))) 5e+03) _returnvalue_3) "TraceTypeQuery1" false 0 "None"))
  (if (== (Game|Player|GetPlayerPawn 0) (.HitActor (Collision|BreakHitResult _outhit)))
    (CallFunction|Attack)
    (CallFunction|GetAnnoyed)
    (elif (>= (Variables|Default|GetscanRotation) 359.0)
      (Variables|Default|SetscanRotation 0.0)
      (else
        (Variables|Default|SetscanRotation (+ (Variables|Default|GetscanRotation) 1.0))))))