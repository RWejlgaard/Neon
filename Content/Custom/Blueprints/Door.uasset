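; A colour-keyed door that vanishes when the player touches it while holding the matching key.
; On BeginPlay, red, green or blue flags pick the glow material for the door mesh and its Key component.
; On box overlap, it casts the player pawn to TopNeon and destroys itself if that pawn has the matching key flag.
; A disconnected Key_DM spawn node never runs.
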(event OnComponentBeginOverlap(Box)
  (params (OverlappedComponent :type Primitive%20Component%20Object%20Reference) (OtherActor :type Actor%20Object%20Reference) (OtherComp :type Primitive%20Component%20Object%20Reference) (OtherBodyIndex :type Integer) (bFromSweep :type Boolean) (SweepResult :type Hit%20Result%20Structure%20%28by%20ref%29))
  (bind _returnvalue (Game|Player|GetPlayerPawn 0))
  (if (== OtherActor _returnvalue)
    (bind _astop_neon (Utilities|Casting|CastToTopNeon _returnvalue)
      (:then
        (if (Variables|Default|GetIsRed)
          (if (Variables|/Game/Custom/Blueprints/TopNeon.TopNeon_C|GetHasRedKey _astop_neon)
            (Actor|DestroyActor :!label _label))
          (elif (Variables|Default|GetIsGreen)
            (if (Variables|/Game/Custom/Blueprints/TopNeon.TopNeon_C|GetHasGreenKey _astop_neon)
              (goto _label))
            (elif (Variables|Default|GetIsBlue)
              (if (Variables|/Game/Custom/Blueprints/TopNeon.TopNeon_C|GetHasBlueKey _astop_neon)
                (goto _label))))))
      (:CastFailed
        (Development|PrintString "CAST TO TOPNEON FAILED")))))

(event EventBeginPlay
  (if (Variables|Default|GetIsRed)
    (Rendering|Material|SetMaterial (Variables|Default|GetKey) 0 "/Game/Custom/Material/RedGlow.RedGlow")
    (Rendering|Material|SetMaterial (Variables|Default|GetStaticMesh) 0 "/Game/Custom/Material/RedGlow.RedGlow")
    (elif (Variables|Default|GetIsGreen)
      (Rendering|Material|SetMaterial (Variables|Default|GetKey) 0 "/Game/Custom/Material/GreenGlow.GreenGlow")
      (Rendering|Material|SetMaterial (Variables|Default|GetStaticMesh) 0 "/Game/Custom/Material/GreenGlow.GreenGlow")
      (elif (Variables|Default|GetIsBlue)
        (Rendering|Material|SetMaterial (Variables|Default|GetKey) 0 "/Game/Custom/Material/BlueGlow.BlueGlow")
        (Rendering|Material|SetMaterial (Variables|Default|GetStaticMesh) 0 "/Game/Custom/Material/BlueGlow.BlueGlow")))))

(event EventTick
  (params (DeltaSeconds :type Float%20%28single-precision%29)))

(fn ConstructionScript)