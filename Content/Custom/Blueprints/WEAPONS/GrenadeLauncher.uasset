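; Grenade projectile actor, named GrenadeLauncher, that explodes on a fixed timer after spawning.
; On BeginPlay it waits a few seconds, swaps the Blast component to a red glow material, applies radial damage with falloff at that component's location, then destroys itself shortly after.
; Impact detonation, AI proximity detection and homing-target logic are left disconnected, so hits and overlaps trigger nothing.
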(event OnComponentHit(Box)
  (params (OtherActor :type Actor%20Object%20Reference) (OtherComp :type Primitive%20Component%20Object%20Reference) (NormalImpulse :type Vector :default "0, 0, 0") (Hit :type Hit%20Result%20Structure%20%28by%20ref%29)))

(event EventBeginPlay
  (bind _blast (Variables|Default|GetBlast))
  (Utilities|FlowControl|Delay 3.0)
  (Rendering|Material|SetMaterial _blast 0 "/Game/Custom/Material/RedGlow.RedGlow")
  (Class|GameplayStatics|ApplyRadialDamagewithFalloff 75.0 7e+01 (Transformation|GetWorldLocation _blast) 1.5e+02 2e+02 0.5 0 0 0 0 "ECC_Visibility")
  (Utilities|FlowControl|Delay 0.15)
  (Actor|DestroyActor))

(event Collision|EventActorBeginOverlap
  (params (OtherActor :type Actor%20Object%20Reference)))

(event EventTick
  (params (DeltaSeconds :type Float%20%28single-precision%29)))

(fn ConstructionScript)